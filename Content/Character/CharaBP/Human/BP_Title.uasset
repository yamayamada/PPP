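; BP_Title is a human character Blueprint, apparently a title-screen variant, that appears with a random skin.
; On BeginPlay it runs parent logic, then calls SetSkin with a random index sized to the game instance's CharMeshArray.
; It then casts its AI controller to AICON_Enemy and switches it to the mode enum's NewEnumerator0 entry.
; Tick and the construction script only defer to the parent.
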(event EventBeginPlay
  (|CallParentFunction)
  (CallFunction|SetSkin (Math|Random|RandomInteger (Utilities|Array|Length (Variables|/Game/GameInstance/MyGameInstance.MyGameInstance_C|GetCharMeshArray (Variables|Default|GetMyGameInstance)))))
  (bind _asaicon_enemy (Utilities|Casting|CastToAICON_Enemy (AI|GetAIController self)))
  (Default|ModeChange _asaicon_enemy "NewEnumerator0"))

(event EventTick
  (params (DeltaSeconds :type Float%20%28single-precision%29))
  (|CallParentFunction DeltaSeconds))

(fn ConstructionScript
  (|CallParentFunction))