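; Player character Blueprint, derived from a parent character class, that starts as the infected, player-operated character.
; BeginPlay sets both state flags, shifts one citizen from non-infected to infected in the game instance, and stores zombie stats (life limit, jump velocity, attack force) there.
; It also debug-prints the mesh material's name and creates a dynamic material instance with MaskLerp fully on.
; Tick and construction only call the parent.
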(event EventBeginPlay
  (bind _mesh (Variables|Character|GetMesh))
  (bind _returnvalue (Rendering|Material|GetMaterial _mesh 0))
  (|CallParentFunction)
  (Variables|Default|SetisOperationPlayer true)
  (Variables|Default|SetisInfection true)
  (Default|SetCitizen (Variables|Default|GetMyGameInstance) (Utilities|Struct|MakeS_CitizenStatus 0.0 -1.0 1.0 0.0))
  (Variables|/Game/GameInstance/MyGameInstance.MyGameInstance_C|SetZombieParameter (Variables|Default|GetMyGameInstance) (Utilities|Struct|MakeS_ZombieParameter 0.0 (Variables|Default|GetDefaultLifeLimit) (Variables|/Script/Engine.CharacterMovementComponent|GetJumpZVelocity (Variables|Character|GetCharacterMovement)) (Variables|Default|GetLastAttackForce)))
  (Development|PrintString (Utilities|GetDisplayName _returnvalue))
  (bind _returnvalue_2 (Rendering|Material|CreateDynamicMaterialInstance _mesh 0 _returnvalue :!class /Script/Engine.PrimitiveComponent))
  (Rendering|Material|SetScalarParameterValue _returnvalue_2 "MaskLerp" 1.0 :!class /Script/Engine.MaterialInstanceDynamic))

(event EventTick
  (params (DeltaSeconds :type Float%20%28single-precision%29))
  (|CallParentFunction DeltaSeconds))

(fn ConstructionScript
  (|CallParentFunction))