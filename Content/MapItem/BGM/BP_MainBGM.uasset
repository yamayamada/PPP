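; Main background music actor that sets its BGM on an audio component and plays it on begin when IsPlay is set.
; When IsMain is set, Tick reads CitizenStatus from the game instance and raises pitch through a curve of the infected-plus-dead share of citizens.
; With infection below one, Tick restarts a timeline that scales the current pitch, stopping audio at 0.1 or lower.
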(event Custom|TLEnd
  (bind _pitch (Timeline|TLPitch Stop)
    (:Update
      (CallFunction|PitchUp (* _pitch (Variables|/Script/Engine.AudioComponent|GetPitchMultiplier (Variables|Default|GetAudio))))
      (if (<= (* _pitch (Variables|/Script/Engine.AudioComponent|GetPitchMultiplier (Variables|Default|GetAudio))) 0.1)
        (Audio|Components|Audio|Stop (Variables|Default|GetAudio))))))

(event Custom|TLStart
  (bind _pitch (Timeline|TLPitch PlayFromStart)
    (:Update
      (CallFunction|PitchUp (* _pitch (Variables|/Script/Engine.AudioComponent|GetPitchMultiplier (Variables|Default|GetAudio))))
      (if (<= (* _pitch (Variables|/Script/Engine.AudioComponent|GetPitchMultiplier (Variables|Default|GetAudio))) 0.1)
        (Audio|Components|Audio|Stop (Variables|Default|GetAudio))))))

(event EventBeginPlay
  (bind _audio (Variables|Default|GetAudio))
  (Audio|Components|Audio|SetSound _audio (Variables|Default|GetBGM))
  (Audio|Components|Audio|Stop _audio)
  (if (Variables|Default|GetisPlay)
    (Audio|Components|Audio|Play (Variables|Default|GetAudio) 0.0)))

(event EventTick
  (params (DeltaSeconds :type Float%20%28single-precision%29))
  (if (Variables|Default|GetisMain)
    (bind _asmy_game_instance (Utilities|Casting|CastToMyGameInstance (Game|GetGameInstance)))
    (if (>= (.infection (Variables|/Game/GameInstance/MyGameInstance.MyGameInstance_C|GetCitizenStatus _asmy_game_instance)) 1.0)
      (CallFunction|PitchUp (+ (Math|Curves|GetFloatValue (Variables|Default|GetPitch) (/ (+ (.infection (Variables|/Game/GameInstance/MyGameInstance.MyGameInstance_C|GetCitizenStatus _asmy_game_instance)) (.dead (Variables|/Game/GameInstance/MyGameInstance.MyGameInstance_C|GetCitizenStatus _asmy_game_instance))) (.citizen (Variables|/Game/GameInstance/MyGameInstance.MyGameInstance_C|GetCitizenStatus _asmy_game_instance)))) 1.0))
      (else
        (CallFunction|TLStart)))))

(fn ConstructionScript)

(fn PitchUp
  (params (NewPitchMultiplier :type Float%20%28single-precision%29))
  (Audio|Components|Audio|SetPitchMultiplier (Variables|Default|GetAudio) NewPitchMultiplier))