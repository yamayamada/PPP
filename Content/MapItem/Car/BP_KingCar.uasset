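; BP_KingCar is a map car that drives along a 2D heading while a BP_Owner overlaps its Box1 trigger.
; Tick moves it and, at intersections, rotates the heading through 90 degrees at a speed set by the intersection's X scale.
; On each BP_Intersection overlap it calls TurnSelect, then alternates between straight and right via TurnFlg.
; Overlapping BP_ParkOut starts a Crash timeline that tilts the car and decays its vertical movement from upward.
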(event OnComponentBeginOverlap(Box)
  (params (OverlappedComponent :type Primitive%20Component%20Object%20Reference) (OtherActor :type Actor%20Object%20Reference) (OtherComp :type Primitive%20Component%20Object%20Reference) (OtherBodyIndex :type Integer) (bFromSweep :type Boolean) (SweepResult :type Hit%20Result%20Structure%20%28by%20ref%29))
  (bind _movevec (Variables|Default|GetmoveVec))
  (bind _asbp_intersection (Utilities|Casting|CastToBP_Intersection OtherActor)
    (:then
      (Default|TurnSelect _asbp_intersection self)
      (if (Variables|Default|GetTurnFlg)
        (CallFunction|InIntersection "NewEnumerator2" (.x (Transformation|GetActorScale3D _asbp_intersection)))
        (else
          (CallFunction|InIntersection "NewEnumerator1" (.x (Transformation|GetActorScale3D _asbp_intersection)))))
      (Variables|Default|SetTurnFlg (not (Variables|Default|GetTurnFlg))))
    (:CastFailed
      (Utilities|Casting|CastToBP_ParkOut OtherActor)
      (Variables|Default|SetCrashMove 1.0)
      (Timeline|Crash PlayFromStart
        (:Update
          (Transformation|SetActorRotation (Math|Rotator|CombineRotators (Transformation|GetActorRotation) (Math|Rotator|MakeRotator (* (.y _movevec) 3.0) (* (.x _movevec) -3.0) 0.0)))
          (Variables|Default|SetCrashMove (- (Variables|Default|GetCrashMove) 0.01)))))))

(event OnComponentBeginOverlap(Box1)
  (params (OverlappedComponent :type Primitive%20Component%20Object%20Reference) (OtherActor :type Actor%20Object%20Reference) (OtherComp :type Primitive%20Component%20Object%20Reference) (OtherBodyIndex :type Integer) (bFromSweep :type Boolean) (SweepResult :type Hit%20Result%20Structure%20%28by%20ref%29))
  (Utilities|Casting|CastToBP_Owner OtherActor)
  (Variables|Default|SetisRide true))

(event OnComponentEndOverlap(Box1)
  (params (OverlappedComponent :type Primitive%20Component%20Object%20Reference) (OtherActor :type Actor%20Object%20Reference) (OtherComp :type Primitive%20Component%20Object%20Reference) (OtherBodyIndex :type Integer))
  (Utilities|Casting|CastToBP_Owner OtherActor)
  (Variables|Default|SetisRide false))

(event EventBeginPlay
  (bind _basespeed (Variables|Default|GetBaseSpeed))
  (Variables|Default|Setpos (Transformation|GetActorLocation))
  (Variables|Default|SetSpeed _basespeed)
  (Variables|Default|SetResetSpeed _basespeed))

(event Collision|EventActorBeginOverlap
  (params (OtherActor :type Actor%20Object%20Reference)))

(event EventTick
  (params (DeltaSeconds :type Float%20%28single-precision%29))
  (bind _returnvalue (Math|Vector2D|MakeVector2D 1.0 0.0))
  (bind _basespeed (Variables|Default|GetBaseSpeed))
  (if (Variables|Default|GetisRide)
    (bind _output_get (Variables|Default|Setpos (+ (Variables|Default|Getpos) (* (Math|Conversions|ToVector(Vector2D) (Variables|Default|GetmoveVec) (Variables|Default|GetCrashMove)) (Variables|Default|GetSpeed)))))
    (Transformation|SetActorLocation _output_get false false)
    (if (Variables|Default|GetIsIntersection)
      (Variables|Default|SetmoveVec (CallFunction|FAddition (Variables|Default|GetmoveVec) (Variables|Default|GetRot)))
      (if (>= (CallFunction|FDot (Variables|Default|GetmoveVec) (Variables|Default|GetBaseVec)) 9e+01)
        (Variables|Default|SetmoveVec (CallFunction|FAddition (Variables|Default|GetBaseVec) (Variables|Default|GetBaseTurn)))
        (Variables|Default|SetIsIntersection false)
        (Variables|Default|SetSpeed _basespeed)
        (Variables|Default|SetResetSpeed _basespeed))
      (Transformation|SetActorRotation (Math|Rotator|MakeRotator 0.0 0.0 (* (CallFunction|FDot (Variables|Default|GetmoveVec) _returnvalue) (CallFunction|FCross (Variables|Default|GetmoveVec) _returnvalue)))))))

(fn ConstructionScript)

(fn InIntersection
  (params (TurnType :type E_TurnType%20Enum :default "NewEnumerator0") (HandleRot :type Float%20%28single-precision%29))
  (bind _returnvalue (* HandleRot 0.5))
  (Variables|Default|SetBaseVec (Variables|Default|GetmoveVec))
  (switch Utilities|FlowControl|Switch|SwitchonE_TurnType TurnType
    (:NewEnumerator0
      (Variables|Default|SetIsIntersection true)
      (Variables|Default|SetResetSpeed _returnvalue)
      (Variables|Default|SetSpeed _returnvalue)
      (Variables|Default|SetBaseTurn -9e+01)
      (Variables|Default|SetRot -1.0))
    (:NewEnumerator2
      (Variables|Default|SetIsIntersection true)
      (Variables|Default|SetResetSpeed HandleRot)
      (Variables|Default|SetSpeed HandleRot)
      (Variables|Default|SetBaseTurn 9e+01)
      (Variables|Default|SetRot 1.0))))

(fn Ride
  (params (flg :type Boolean))
  (Variables|Default|SetisRide flg))