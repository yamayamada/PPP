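; BP_Intersection is a car-map intersection actor that picks a random turn type for a car.
; BeginPlay builds an array of open-direction flags from its North, East, South and West settings.
; TurnSelect finds the car's side using 2D cross and dot helpers bucketed by 45, then rerolls a wrapped direction offset until it hits an enabled flag.
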(event EventBeginPlay
  (bind _direction (Variables|Default|GetDirection))
  (Variables|Default|SetDirectionFlg (Utilities|Array|MakeArray (.north _direction) (.east _direction) (.south _direction) (.west _direction))))

(event Collision|EventActorBeginOverlap
  (params (OtherActor :type Actor%20Object%20Reference)))

(event EventTick
  (params (DeltaSeconds :type Float%20%28single-precision%29)))

(fn ConstructionScript)

(fn TurnSelect
  (params (car :type Actor%20Object%20Reference))
  (bind _directionflg (Variables|Default|GetDirectionFlg))
  (bind _returnvalue (Utilities|Array|Length _directionflg))
  (LocalVariables|SetActorDirection (CallFunction|IntersectiontoCarDirection car))
  (while (LocalVariables|GetloopBreak)
    (LocalVariables|SetTurnTypeNum (Math|Random|RandomIntegerinRange 1 3))
    (if (< (+ (Math|Conversions|ToInteger(Byte) (LocalVariables|GetActorDirection)) (LocalVariables|GetTurnTypeNum)) _returnvalue)
      (LocalVariables|SetloopBreak (not (Utilities|Array|Get(acopy) (Variables|Default|GetDirectionFlg) (+ (Math|Conversions|ToInteger(Byte) (LocalVariables|GetActorDirection)) (LocalVariables|GetTurnTypeNum)))))
      (else
        (LocalVariables|SetloopBreak (not (Utilities|Array|Get(acopy) (Variables|Default|GetDirectionFlg) (- (+ (Math|Conversions|ToInteger(Byte) (LocalVariables|GetActorDirection)) (LocalVariables|GetTurnTypeNum)) _returnvalue)))))))
  (return (Utilities|Enum|ByteToEnumE_TurnType (Math|Conversions|ToByte(Integer) (- (LocalVariables|GetTurnTypeNum) 1)))))

(fn IntersectiontoCarDirection
  (params (Caｒ :type Actor%20Object%20Reference))
  (bind _returnvalue (Transformation|GetActorLocation))
  (bind _returnvalue_2 (Math|Vector2D|MakeVector2D 1.0 0.0))
  (bind _returnvalue_3 (Math|Conversions|ToVector2D(Vector) _returnvalue))
  (bind _returnvalue_4 (Transformation|GetActorLocation Caｒ))
  (bind _returnvalue_5 (Math|Conversions|ToVector2D(Vector) _returnvalue_4))
  (bind _returnvalue_6 (- _returnvalue_5 _returnvalue_3))
  (bind _returnvalue_7 (Math|Vector2D|Normalize2D _returnvalue_6))
  (switch int (Math|Float|Truncate (/ (* (CallFunction|FCross2 _returnvalue_2 _returnvalue_7) (CallFunction|FDot2 _returnvalue_2 _returnvalue_7)) 45.0))
    (:Default
      (Development|PrintString "ERROR"))
    (:-3
      _)
    (:-2
      (return "NewEnumerator1"))
    (:-1
      (return "NewEnumerator1"))
    (:0
      (return "NewEnumerator0"))
    (:1
      (return "NewEnumerator3"))
    (:2
      (return "NewEnumerator3"))
    (:3
      _))
  (return "NewEnumerator2"))