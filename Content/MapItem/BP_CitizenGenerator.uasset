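; BP_CitizenGenerator is a placed or spawned actor that creates a citizen AI on low-lying ground beneath it.
; On BeginPlay it moves to a high altitude, line traces down, and spawns BP_Human with BT_Citizen at the impact point if below a height limit.
; CoordinateObservation generalizes this probe for a given point and limits, returning validity and coordinates with a fixed Z, but is not called within this Blueprint.
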(event EventBeginPlay
  (bind _returnvalue (Transformation|GetActorLocation))
  (bind _returnvalue_2 (Transformation|GetActorLocation))
  (Transformation|SetActorLocation (Math|Vector|MakeVector (.x _returnvalue) (.y _returnvalue) 4e+03) false false)
  (bind _outhit (Collision|LineTraceByChannel _returnvalue_2 (+ _returnvalue_2 (* (Math|Vector|MakeVector 0.0 0.0 -1.0) 4e+03)) "TraceTypeQuery1" false 0 "None"))
  (if (<= (.Z (Math|Vector|BreakVector (.ImpactPoint (Collision|BreakHitResult _outhit)))) 1.5e+02)
    (AI|SpawnAIFromClass "/Game/Character/CharaBP/Human/BP_Human.BP_Human_C" "/Game/AI/BB_BT/BT_Citizen.BT_Citizen" (.ImpactPoint (Collision|BreakHitResult _outhit)) "0, 0, 0" false)))

(event Collision|EventActorBeginOverlap
  (params (OtherActor :type Actor%20Object%20Reference)))

(event EventTick
  (params (DeltaSeconds :type Float%20%28single-precision%29)))

(fn ConstructionScript)

(fn CoordinateObservation
  (params (ObservationPoint :type Vector) (UpperLimit :type Float%20%28single-precision%29) (SpawnLimit :type Float%20%28single-precision%29))
  (bind (_x _y) (Math|Vector|BreakVector ObservationPoint))
  (bind _returnvalue (Transformation|GetActorLocation))
  (Transformation|SetActorLocation (Math|Vector|MakeVector _x _y UpperLimit) false false)
  (bind _outhit (Collision|LineTraceByChannel _returnvalue (+ _returnvalue (* (Math|Vector|MakeVector 0.0 0.0 -1.0) UpperLimit)) "TraceTypeQuery1" false 0 "None"))
  (return (<= (.Z (Math|Vector|BreakVector (.ImpactPoint (Collision|BreakHitResult _outhit)))) SpawnLimit) (Math|Vector|MakeVector (.X (Math|Vector|BreakVector (.ImpactPoint (Collision|BreakHitResult _outhit)))) (.Y (Math|Vector|BreakVector (.ImpactPoint (Collision|BreakHitResult _outhit)))) 2e+02)))